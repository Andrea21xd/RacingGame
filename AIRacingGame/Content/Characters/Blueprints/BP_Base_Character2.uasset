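; BP_Base_Character2 is a character Blueprint that appears to be an unfinished prototype for spline-following movement.
; Tick advances SplineProgress by Speed and delta time while SplineRef is valid, otherwise it prints a warning.
; The Sequence after that update drives nothing, so the actor is not moved by this graph.
; Disconnected experiments remain for placing the actor along Spline0 or Spline1 and for pushing or repositioning the Cylinder.
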(event `self.ReceiveTick`
  (params (DeltaSeconds :type "Float (single-precision)"))
  (`/Engine/EditorBlueprintResources/StandardMacros.IsValid` (`self.SplineRef`)
    (:`Is Valid`
      (bind _output_get (set `self.SplineProgress` (+ (* DeltaSeconds (`self.Speed`)) (`self.SplineProgress`))))
      (`|ExecutionSequence`))
    (:`Is Not Valid`
      (`KismetSystemLibrary.PrintString` "SplineRef is not set!"))))

(fn `UserConstructionScript`)
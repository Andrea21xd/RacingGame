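; BP_base_Character is a base character that travels automatically along a referenced spline.
; Each Tick advances SplineProgress by Speed and delta time, places the actor at that world location plus Offset, and applies the spline's local-space rotation.
; It prints a warning while SplineRef is unset.
; Disconnected leftover nodes hold unused experiments with forward force and left/right movement along a second CharSpline.
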(event `self.ReceiveTick`
  (params (DeltaSeconds :type "Float (single-precision)"))
  ; Main Logic
  (`|ExecutionSequence`
    (:`then_0`
      (`/Engine/EditorBlueprintResources/StandardMacros.IsValid` (`self.SplineRef`)
        (:`Is Valid`
          (bind _output_get (set `self.SplineProgress` (+ (* DeltaSeconds (`self.Speed`)) (`self.SplineProgress`))))
          (`|ExecutionSequence`
            (:`then_0`
              (`self.K2_SetActorLocation` (+ (`SplineComponent.GetLocationAtDistanceAlongSpline` (`/Game/Characters/Blueprints/BP_Spline.Spline0` (`self.SplineRef`)) _output_get "World") (`self.Offset`))))
            (:`then_1`
              (`self.K2_SetActorRotation` (`SplineComponent.GetRotationAtDistanceAlongSpline` (`/Game/Characters/Blueprints/BP_Spline.Spline0` (`self.SplineRef`)) _output_get "Local")))))
        (:`Is Not Valid`
          (`KismetSystemLibrary.PrintString` "SplineRef is not set!" true true (struct :`G` 0.66 :`B` 1.0 :`A` 1.0) 10.0))))))

(fn `UserConstructionScript`)